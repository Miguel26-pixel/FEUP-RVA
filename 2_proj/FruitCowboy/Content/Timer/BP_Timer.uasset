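; BP_Timer is a countdown clock that shows minutes and seconds on text components and ends a fruit round when it runs out.
; StartClock runs a looping one-second timer whose TickClock decrements the time and refreshes the display, while StopClock pauses it.
; At zero it pauses the timer and despawns every BP_Fruit actor.
; ResetClock sets a new time without refreshing the display, which is also updated on construction.
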(event `StopClock`
  (`KismetSystemLibrary.K2_PauseTimerHandle` (`self.TimerHandle`)))

(event `StartClock`
  (bind _returnvalue (`KismetSystemLibrary.K2_SetTimerDelegate` (delegate `TickClock`) 1.0 true))
  (set `self.TimerHandle` _returnvalue))

(event `TickClock`
  (if (== (`self.Sec`) 0)
    (if (== (`self.Min`) 0)
      (`KismetSystemLibrary.K2_PauseTimerHandle` (`self.TimerHandle`))
      (`KismetSystemLibrary.PrintString` "Timer Finished")
      (bind _outactors (`GameplayStatics.GetAllActorsOfClass` "/Game/Fruit/BP_Fruit.BP_Fruit_C"))
      (for _array_element _outactors
        (`/Game/Fruit/BP_Fruit.Despawn` _array_element))
      (`KismetSystemLibrary.PrintString` "All fruits destroyed")
      (else
        (set `self.Sec` 59)
        (set `self.Min` (- (`self.Min`) 1))
        (`self.UpdateTimeDisplay` :!label _label)))
    (else
      (set `self.Sec` (- (`self.Sec`) 1))
      (goto _label))))

(fn `ResetClock`
  (params (Minutes :type Integer) (Seconds :type Integer))
  (set `self.Min` Minutes)
  (set `self.Sec` Seconds))

(fn `UpdateTimeDisplay`
  (`TextRenderComponent.K2_SetText` (`self.MinutesText`) (`KismetTextLibrary.Conv_IntToText` (`self.Min`) false true 2 3))
  (`TextRenderComponent.K2_SetText` (`self.SecondsText`) (`KismetTextLibrary.Conv_IntToText` (`self.Sec`) false true 2 2)))

(fn `UserConstructionScript`
  (`self.UpdateTimeDisplay`))