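; BP_ChallengePlatform is a platform that starts its linked Challenge when a VRPawn enters its trigger Box and stops it when the pawn leaves.
; On BeginPlay it creates a dynamic material from M_Platform on the Cube with brightness off.
; Overlaps toggle the material's Bright parameter and play or reverse FlashTimeline, which drives its Opacity for visual feedback.
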(event `self.ReceiveBeginPlay`
  (bind _returnvalue (`PrimitiveComponent.CreateDynamicMaterialInstance` (`self.Cube`) 0 "/Game/Challenges/Materials/M_Platform.M_Platform" "None"))
  (bind _output_get (set `self.PlatformMaterial` _returnvalue))
  (`MaterialInstanceDynamic.SetScalarParameterValue` _output_get "Bright" 0.0))

(event `self.Box.OnComponentBeginOverlap`
  (params (OverlappedComponent :type "PrimitiveComponent Object Reference") (OtherActor :type "Actor Object Reference") (OtherComp :type "PrimitiveComponent Object Reference") (OtherBodyIndex :type Integer) (bFromSweep :type Boolean) (SweepResult :type "HitResult Structure (by ref)"))
  (cast `/Game/VRTemplate/Blueprints/VRPawn` OtherActor)
  (`/Game/Challenges/BP_Challenge.Start` (`self.Challenge`))
  (`MaterialInstanceDynamic.SetScalarParameterValue` (`self.PlatformMaterial`) "Bright" 1.0)
  (bind (_direction _opacity) (`Timeline|FlashTimeline` :!label _label)
    (:`Update`
      (`MaterialInstanceDynamic.SetScalarParameterValue` (`self.PlatformMaterial`) "Opacity" _opacity))))

(event `self.Box.OnComponentEndOverlap`
  (params (OverlappedComponent :type "PrimitiveComponent Object Reference") (OtherActor :type "Actor Object Reference") (OtherComp :type "PrimitiveComponent Object Reference") (OtherBodyIndex :type Integer))
  (cast `/Game/VRTemplate/Blueprints/VRPawn` OtherActor)
  (`/Game/Challenges/BP_Challenge.Stop` (`self.Challenge`))
  (`MaterialInstanceDynamic.SetScalarParameterValue` (`self.PlatformMaterial`) "Bright" 0.0)
  (goto _label :!via `Reverse`))

(fn `UserConstructionScript`)