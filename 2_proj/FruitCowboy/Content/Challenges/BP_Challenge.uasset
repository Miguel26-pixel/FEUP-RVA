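; BP_Challenge is a challenge controller that starts and stops a gameplay challenge through its Start and Stop events.
; Start activates its spawners, makes its disappearing walls vanish and, if timed, resets and starts the timer display with the configured minutes and seconds.
; Stop halts spawning and restores the walls; for timed challenges it also stops the clock and destroys every BP_Fruit actor in the world.
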(event `Start`
  (bind _timerdisplay (`self.TimerDisplay`))
  (for _array_element (`self.Spawners`)
    (`/Game/Fruit/BP_FruitSpawner.StartSpawning` _array_element))
  (for _array_element_2 (`self.DisapearingWalls`)
    (`/Game/Challenges/BP_DisapearingWall.Disapear` _array_element_2))
  (if (`self.IsTimed`)
    (`/Game/Timer/BP_Timer.ResetClock` _timerdisplay (`self.Minutes`) (`self.Seconds`))
    (`/Game/Timer/BP_Timer.StartClock` _timerdisplay)))

(event `Stop`
  (for _array_element (`self.Spawners`)
    (`/Game/Fruit/BP_FruitSpawner.StopSpawning` _array_element))
  (for _array_element_2 (`self.DisapearingWalls`)
    (`/Game/Challenges/BP_DisapearingWall.Appear` _array_element_2))
  (if (`self.IsTimed`)
    (`/Game/Timer/BP_Timer.StopClock` (`self.TimerDisplay`))
    (bind _outactors (`GameplayStatics.GetAllActorsOfClass` "/Game/Fruit/BP_Fruit.BP_Fruit_C"))
    (for _array_element_3 _outactors
      (`self.K2_DestroyActor` _array_element_3))))

(fn `UserConstructionScript`)