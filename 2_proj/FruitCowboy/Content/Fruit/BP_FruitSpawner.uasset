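; BP_FruitSpawner spawns waves of BP_Fruit actors, started and halted through the StartSpawning and StopSpawning events.
; Each wave spawns a random number of fruit, each with a random FruitData entry, at random offsets around a point ahead of the spawner.
; A breakable loop re-enters itself after a delay to repeat waves, while StopSpawning sets a flag and breaks it.
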(event `self.ReceiveBeginPlay`)

(event `StartSpawning`
  (set `self.Stop` false)
  (for _ (range (+ (`KismetMathLibrary.RandomIntegerInRange` (`self.MinNumberFruitPerWave`) (`self.MaxNumberFruitPerWave`)) 1)) :!label _label
    (bind (_randomoffsetdirection _returnvalue) (`self.GetRandomSpawnLocation`))
    (`|SpawnActorFromClass` "/Game/Fruit/BP_Fruit.BP_Fruit_C" (`KismetMathLibrary.MakeTransform` _returnvalue) "AdjustIfPossibleButAlwaysSpawn" "MultiplyWithRoot" null (`KismetArrayLibrary.Array_Random` (`self.FruitData`)) 0 null))
  (if (not (`self.Stop`))
    (`KismetSystemLibrary.Delay` (`self.FruitSpawnDelay`))
    (goto _label)))

(event `StopSpawning`
  (set `self.Stop` true)
  (goto _label :!via `Break`))

(fn `GetRandomSpawnLocation`
  (returns (RandomOffsetDirection :type "Vector Structure") (ReturnValue :type "Vector Structure"))
  (bind _returnvalue (`KismetMathLibrary.RandomUnitVector`))
  (return _returnvalue (+ (+ (`self.K2_GetActorLocation`) (* (`self.GetActorForwardVector`) (`self.SpawnRange`))) (* _returnvalue (`KismetMathLibrary.RandomFloatInRange` 0.0 (`self.RandomSpawnOffset`))))))

(fn `UserConstructionScript`)